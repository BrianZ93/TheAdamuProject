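; Player start actor for AdamuProject that spawns a player's main building and a starting worker based on the selected race.
; SpawnMainBuildingandWorkers picks the race's building class (Human or Apkallu, both using BP_Caveman workers) and line-traces down to find the ground.
; The game mode's GameplayManager spawns the building into its pool for player 0, then SpawnWorkers traces from an offset beside it to spawn one worker the same way.
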(event EventBeginPlay)

(event EventTick
  (params (DeltaSeconds :type Float%20%28single-precision%29)))

(event EventSpawnMainBuildingandWorkers
  (bind _self self)
  (bind _self_2 self)
  (bind _returnvalue (Transformation|GetActorTransform _self_2))
  (bind _location (Math|Transform|BreakTransform _returnvalue))
  (bind _location_2 (Math|Transform|BreakTransform _returnvalue))
  (switch Utilities|FlowControl|Switch|SwitchonERaceType (Variables|Default|GetSelectedRace _self)
    (:Human
      (Variables|Default|SetWorkersToCreate "/Game/Races/Human/Units/Caveman/BP_Caveman.BP_Caveman_C")
      (Variables|Default|SetMainBuildingToCreate (.buildingclass (Variables|Default|GetHumanConfig _self))))
    (:Apkallu
      (Variables|Default|SetWorkersToCreate "/Game/Races/Human/Units/Caveman/BP_Caveman.BP_Caveman_C")
      (Variables|Default|SetMainBuildingToCreate (.buildingclass (Variables|Default|GetApkalluConfig _self)))))
  (bind (_outhit _returnvalue_2) (Collision|LineTraceByChannel (Math|Vector|MakeVector (.x _location) (.y _location) (+ (.z _location) 5e+02)) (Math|Vector|MakeVector (.x _location_2) (.y _location_2) (- (.z _location_2) 1e+04)) "TraceTypeQuery1" false 0 "ForDuration"))
  (if _returnvalue_2
    (bind _asadamu_project_game_mode_base (Utilities|Casting|CastToAdamuProjectGameModeBase (Game|GetGameMode))
      (:then
        (if (Utilities|IsValid (Variables|/Script/TheAdamuProject.AdamuProjectGameModeBase|GetGameplayManager _asadamu_project_game_mode_base))
          (bind _returnvalue_3 (Class|RTSGameplayManager|SpawnActorandAddtoPool (Variables|/Script/TheAdamuProject.AdamuProjectGameModeBase|GetGameplayManager _asadamu_project_game_mode_base) (Variables|Default|GetMainBuildingToCreate) (Math|Conversions|ToTransform(Vector) (.Location (Collision|BreakHitResult _outhit))) (Game|GetPlayerController 0)))
          (CallFunction|SpawnWorkers _returnvalue_3)
          (else
            (Development|PrintString "Gameplay Maanger object is not valid"))))
      (:CastFailed
        (Development|PrintString "Failed to cast to AdamuProjectGameModeBase")))
    (else
      (Development|PrintString "Line Trace could not find spawn location"))))

(fn ConstructionScript)

(fn SpawnWorkers
  (params (MainBuilding :type Actor%20Object%20Reference))
  (bind _returnvalue (Transformation|GetActorTransform MainBuilding))
  (bind _location (Math|Transform|BreakTransform _returnvalue))
  (bind _location_2 (Math|Transform|BreakTransform _returnvalue))
  (bind (_outhit _returnvalue_2) (Collision|LineTraceByChannel (Math|Vector|MakeVector (- (.x _location) 5e+02) (.y _location) (+ (.z _location) 5e+02)) (Math|Vector|MakeVector (.x _location_2) (.y _location_2) (- (.z _location_2) 1e+04)) "TraceTypeQuery1" false 0 "Persistent"))
  (if _returnvalue_2
    (bind _asadamu_project_game_mode_base (Utilities|Casting|CastToAdamuProjectGameModeBase (Game|GetGameMode)))
    (Class|RTSGameplayManager|SpawnActorandAddtoPool (Variables|/Script/TheAdamuProject.AdamuProjectGameModeBase|GetGameplayManager _asadamu_project_game_mode_base) (Variables|Default|GetWorkersToCreate) (Math|Conversions|ToTransform(Vector) (.Location (Collision|BreakHitResult _outhit))) (Game|GetPlayerController 0))))